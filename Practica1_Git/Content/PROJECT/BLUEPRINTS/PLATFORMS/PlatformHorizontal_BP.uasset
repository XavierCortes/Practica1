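; Horizontal moving platform that shuttles its Cube component back and forth between two world-space limits.
; Each Tick offsets the cube along world X or Y, chosen by MovAxis, at a fixed speed scaled by delta time and Direction.
; Direction flips sign when the cube reaches MaxRight or MaxLeft, which serve as the bounds for either axis.
; Movement sets the location directly, without sweep.
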(event `self.ReceiveTick`
  (params (DeltaSeconds :type "Float (single-precision)"))
  (bind _returnvalue_x (`KismetMathLibrary.BreakVector` (`SceneComponent.K2_GetComponentLocation` (`self.Cube`))))
  (bind (_returnvalue_x_2 _returnvalue_y) (`KismetMathLibrary.BreakVector` (`SceneComponent.K2_GetComponentLocation` (`self.Cube`))))
  (bind (_returnvalue_x_3 _returnvalue_y_2) (`KismetMathLibrary.BreakVector` (`SceneComponent.K2_GetComponentLocation` (`self.Cube`))))
  (bind _returnvalue_x_4 (`KismetMathLibrary.BreakVector` (`SceneComponent.K2_GetComponentLocation` (`self.Cube`))))
  (if (`KismetStringLibrary.EqualEqual_StrStr` (`self.MovAxis`) "X")
    (if (> (`self.Direction`) 0)
      (if (< _returnvalue_x_4 (`self.MaxRight`))
        (`SceneComponent.K2_SetWorldLocation` (`self.Cube`) (+ (`SceneComponent.K2_GetComponentLocation` (`self.Cube`)) (* (* (80.0 0.0 0.0) (`GameplayStatics.GetWorldDeltaSeconds`)) (`self.Direction`))) false false :!label _label)
        (else
          (set `self.Direction` (* (`self.Direction`) -1))))
      (elif (> _returnvalue_x (`self.MaxLeft`))
        (goto _label)
        (else
          (set `self.Direction` (* (`self.Direction`) -1)))))
    (elif (> (`self.Direction`) 0)
      (if (< _returnvalue_y_2 (`self.MaxRight`))
        (`SceneComponent.K2_SetWorldLocation` (`self.Cube`) (+ (`SceneComponent.K2_GetComponentLocation` (`self.Cube`)) (* (* (0.0 80.0 0.0) (`GameplayStatics.GetWorldDeltaSeconds`)) (`self.Direction`))) false false :!label _label_2)
        (else
          (set `self.Direction` (* (`self.Direction`) -1))))
      (elif (> _returnvalue_y (`self.MaxLeft`))
        (goto _label_2)
        (else
          (set `self.Direction` (* (`self.Direction`) -1)))))))

(fn `UserConstructionScript`)