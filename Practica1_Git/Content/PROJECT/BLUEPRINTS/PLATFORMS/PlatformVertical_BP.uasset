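; Vertical moving platform that travels at constant speed between a minimum and maximum height.
; Tick moves the Cube by delta time and Direction, flipping Direction at each limit.
; Automatic platforms cycle continuously, while others cycle only while the Collider's overlap flag marks the player as aboard.
; After the overlap ends, a non-automatic platform waits three seconds, then descends to its minimum height.
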(event `self.Collider.OnComponentEndOverlap`
  (params (OverlappedComponent :type "PrimitiveComponent Object Reference") (OtherActor :type "Actor Object Reference") (OtherComp :type "PrimitiveComponent Object Reference") (OtherBodyIndex :type Integer))
  (set `self.IsPlayerOn` false)
  (set `self.Timer` 0.0))

(event `self.Collider.OnComponentBeginOverlap`
  (params (OverlappedComponent :type "PrimitiveComponent Object Reference") (OtherActor :type "Actor Object Reference") (OtherComp :type "PrimitiveComponent Object Reference") (OtherBodyIndex :type Integer) (bFromSweep :type Boolean) (SweepResult :type "HitResult Structure (by ref)"))
  (set `self.IsPlayerOn` true))

(event `self.ReceiveTick`
  (params (DeltaSeconds :type "Float (single-precision)"))
  (bind (_returnvalue_x _returnvalue_y _returnvalue_z) (`KismetMathLibrary.BreakVector` (`SceneComponent.K2_GetComponentLocation` (`self.Cube`))))
  (bind (_returnvalue_x_2 _returnvalue_y_2 _returnvalue_z_2) (`KismetMathLibrary.BreakVector` (`SceneComponent.K2_GetComponentLocation` (`self.Cube`))))
  (bind (_returnvalue_x_3 _returnvalue_y_3 _returnvalue_z_3) (`KismetMathLibrary.BreakVector` (`SceneComponent.K2_GetComponentLocation` (`self.Cube`))))
  (if (`self.isAutomatic`)
    (if (> (`self.Direction`) 0) :!label _label
      (if (< _returnvalue_z_3 (`self.MaxHeight`))
        (`SceneComponent.K2_SetWorldLocation` (`self.Cube`) (+ (`SceneComponent.K2_GetComponentLocation` (`self.Cube`)) (* (* (0.0 0.0 80.0) (`GameplayStatics.GetWorldDeltaSeconds`)) (`self.Direction`))) false false :!label _label_2)
        (else
          (set `self.Direction` (* (`self.Direction`) -1))))
      (elif (> _returnvalue_z_2 (`self.MinHeight`))
        (goto _label_2)
        (else
          (set `self.Direction` (* (`self.Direction`) -1)))))
    (elif (`self.IsPlayerOn`)
      (goto _label)
      (elif (>= (`self.Timer`) 3.0)
        (set `self.Direction` -1)
        (if (> _returnvalue_z (`self.MinHeight`))
          (goto _label_2))
        (else
          (set `self.Timer` (+ (`self.Timer`) (`GameplayStatics.GetWorldDeltaSeconds`))))))))

(fn `UserConstructionScript`)