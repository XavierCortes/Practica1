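; AI-controlled NPC character that runs the BT_NPC behavior tree and displays a health bar.
; On BeginPlay it starts the tree and sets up physical animation below the pelvis, so those bones simulate physics while being driven toward the animated pose for partial active ragdoll.
; Every Tick it casts the EnemyHealthBar widget to NPClifebar and pushes Life scaled down by 100 as the bar value.
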(event `self.ReceiveBeginPlay`
  (bind _physicalanimation (`self.PhysicalAnimation`))
  (bind _pelvis (`self.pelvis`))
  (`AIController.RunBehaviorTree` (`AIBlueprintHelperLibrary.GetAIController` self) "/Game/PROJECT/BLUEPRINTS/IA/BT_NPC.BT_NPC")
  ;[1 1 1] Ragdoll IA
  (`PhysicalAnimationComponent.SetSkeletalMeshComponent` _physicalanimation (`self.Mesh`))
  (`PhysicalAnimationComponent.ApplyPhysicalAnimationSettingsBelow` _physicalanimation _pelvis (make `PhysicalAnimationData` false 1000.0 100.0 1000.0 100.0) false)
  (`SkeletalMeshComponent.SetAllBodiesBelowSimulatePhysics` (`self.Mesh`) _pelvis true false))

(event `self.ReceiveTick`
  (params (DeltaSeconds :type "Float (single-precision)"))
  (bind _asnpclifebar (cast `/Game/PROJECT/BLUEPRINTS/IA/NPClifebar` (`WidgetComponent.GetUserWidgetObject` (`self.EnemyHealthBar`))))
  (set `/Game/PROJECT/BLUEPRINTS/IA/NPClifebar.Life_NPC` (/ (`self.Life`) 100.0) _asnpclifebar))

(fn `UserConstructionScript`)