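; Door actor that slides vertically and opens through linked lights, a key, coins or proximity, checked in that priority.
; Tick moves the door toward its height limits, lowering it only in proximity mode.
; Linked lights must all report IsOk, via CheckAllLights.
; Key and coin doors poll the character's E press while overlap sets PlayerIsNear, then deduct the cost and latch CanOpen.
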(event `self.ReceiveTick`
  (params (DeltaSeconds :type "Float (single-precision)"))
  (bind (_returnvalue_x _returnvalue_y _returnvalue_z) (`KismetMathLibrary.BreakVector` (`SceneComponent.K2_GetComponentLocation` (`self.Door`))))
  (bind (_returnvalue_x_2 _returnvalue_y_2 _returnvalue_z_2) (`KismetMathLibrary.BreakVector` (`SceneComponent.K2_GetComponentLocation` (`self.Door`))))
  (bind _returnvalue (> (`KismetArrayLibrary.Array_Length` (`self.remoteLightsL`)) 0))
  (bind _isok (`self.checkAllLights`))
  (if (and _isok _returnvalue)
    (if (< _returnvalue_z (`self.MaxHeight`)) :!label _label
      (`SceneComponent.K2_SetWorldLocation` (`self.Door`) (+ (`SceneComponent.K2_GetComponentLocation` (`self.Door`)) (* (0.0 0.0 100.0) (`GameplayStatics.GetWorldDeltaSeconds`))) false false))
    (elif _returnvalue
      _
      (elif (`self.NeedsKey`)
        (if (`self.CanOpen`)
          (goto _label)
          (elif (`self.PlayerIsNear`)
            (bind _asthird_person_character (cast `/Game/ThirdPersonBP/Blueprints/ThirdPersonCharacter` (`GameplayStatics.GetPlayerPawn` 0)))
            (if (`/Game/ThirdPersonBP/Blueprints/ThirdPersonCharacter.E IsPressed` _asthird_person_character)
              (bind _asthird_person_character_2 (cast `/Game/ThirdPersonBP/Blueprints/ThirdPersonCharacter` (`GameplayStatics.GetPlayerPawn` 0)))
              (if (> (`/Game/ThirdPersonBP/Blueprints/ThirdPersonCharacter.Keys` _asthird_person_character_2) 0)
                (set `self.CanOpen` true)
                (bind _asthird_person_character_3 (cast `/Game/ThirdPersonBP/Blueprints/ThirdPersonCharacter` (`GameplayStatics.GetPlayerPawn` 0)))
                (set `/Game/ThirdPersonBP/Blueprints/ThirdPersonCharacter.Keys` (- (`/Game/ThirdPersonBP/Blueprints/ThirdPersonCharacter.Keys` _asthird_person_character_3) 1) _asthird_person_character_3)))))
        (elif (`self.NeedsCoins`)
          (if (`self.CanOpen`)
            (goto _label)
            (elif (`self.PlayerIsNear`)
              (bind _asthird_person_character_4 (cast `/Game/ThirdPersonBP/Blueprints/ThirdPersonCharacter` (`GameplayStatics.GetPlayerPawn` 0)))
              (if (`/Game/ThirdPersonBP/Blueprints/ThirdPersonCharacter.E IsPressed` _asthird_person_character_4)
                (bind _asthird_person_character_5 (cast `/Game/ThirdPersonBP/Blueprints/ThirdPersonCharacter` (`GameplayStatics.GetPlayerPawn` 0)))
                (if (>= (`/Game/ThirdPersonBP/Blueprints/ThirdPersonCharacter.Coins` _asthird_person_character_5) 5)
                  (set `self.CanOpen` true)
                  (bind _asthird_person_character_6 (cast `/Game/ThirdPersonBP/Blueprints/ThirdPersonCharacter` (`GameplayStatics.GetPlayerPawn` 0)))
                  (set `/Game/ThirdPersonBP/Blueprints/ThirdPersonCharacter.Coins` (- (`/Game/ThirdPersonBP/Blueprints/ThirdPersonCharacter.Coins` _asthird_person_character_6) 5) _asthird_person_character_6)))))
          (elif (`self.PlayerIsNear`)
            (goto _label)
            (elif (> _returnvalue_z_2 (`self.MinHeight`))
              (`SceneComponent.K2_SetWorldLocation` (`self.Door`) (- (`SceneComponent.K2_GetComponentLocation` (`self.Door`)) (* (0.0 0.0 100.0) (`GameplayStatics.GetWorldDeltaSeconds`))) false false))))))))

(event `self.ReceiveActorBeginOverlap`
  (params (OtherActor :type "Actor Object Reference"))
  (set `self.PlayerIsNear` true))

(event `self.ReceiveActorEndOverlap`
  (params (OtherActor :type "Actor Object Reference"))
  (set `self.PlayerIsNear` false))

(fn `checkAllLights`
  (returns (isOK :type Boolean))
  (for _array_element (`self.remoteLightsL`)
    (if (not (`/Game/Geometry/RemoteLight.isOk` _array_element))
      (return false)))
  (return true))

(fn `UserConstructionScript`)